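; Physics-driven catapult that the player character can fire, reset and reload.
; Execute, gated on the character's InteractType, either swings the Arm by retargeting the Spring constraint's angular drive and waking the body, or eases it back to the cocked rotation.
; Reload spawns a scaled-down actor at StoneSpawnPoint, once per shot and only while ready to fire.
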(event `self.ReceiveBeginPlay`
  (`|ExecutionSequence`
    (:`then_0`
      (bind _asbp_third_person_character (cast `/Game/ThirdPerson/Blueprints/BP_ThirdPersonCharacter` (`GameplayStatics.GetPlayerCharacter` 0)))
      (set `self.BPThirdPersonCharacter` _asbp_third_person_character))
    (:`then_1`
      (`SceneComponent.K2_SetWorldRotation` (`self.Arm`) (`KismetMathLibrary.TransformRotation` (`self.GetTransform`) (struct :`Yaw` 90.0)) false false))))

(event `/Game/Catapult/Blueprints/Interfaces/BPI_Execute.Execute`
  (bind _arm (`self.Arm`))
  (if (`|EnumEquality` (`/Game/ThirdPerson/Blueprints/BP_ThirdPersonCharacter.InteractType` (`self.BPThirdPersonCharacter`)) "NewEnumerator0")
    (if (`self.ReadyToFire`)
      (`PhysicsConstraintComponent.SetAngularOrientationTarget` (`self.Spring`) (`KismetMathLibrary.MakeRotator` 0.0 65.0))
      (`PrimitiveComponent.WakeRigidBody` (`self.Arm`) "None")
      (set `self.IsReloaded` false)
      (set `self.ReadyToFire` false)
      (else
        (`PhysicsConstraintComponent.SetAngularOrientationTarget` (`self.Spring`) (`KismetMathLibrary.MakeRotator` 0.0 0.0))
        (`KismetSystemLibrary.MoveComponentTo` _arm (`SceneComponent.RelativeLocation` _arm) (struct :`Yaw` 90.0) true true 2.0)
        (set `self.ReadyToFire` true)))))

(event `/Game/Catapult/Blueprints/Interfaces/BPI_CatapultReload.Reload`
  (if (`self.ReadyToFire`)
    (if (not (`self.IsReloaded`))
      (`|SpawnActorFromClass` "/Game/Catapult/Blueprints/BP_Stone.BP_Stone_C" (`KismetMathLibrary.MakeTransform` (`SceneComponent.K2_GetComponentLocation` (`self.StoneSpawnPoint`)) (struct) (0.2 0.2 0.2)) "Undefined" "OverrideRootScale" null null)
      (set `self.IsReloaded` true))))

(fn `UserConstructionScript`)